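; DeathEffect_BP is a death effect that bursts a cloud of physics-driven mesh debris from a given transform.
; Its Emit event spawns a hundred DeathParticleMesh_BP actors at that location and rotation, sized by Scale.
; Each cube gets a random velocity along a vertical cone, with Spread setting signed speed and Height stretching the Z component, plus a random spin.
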(event Custom|Emit
  (params (SpawnTransform :type Transform))
  (bind _scale (Variables|Default|GetScale))
  (bind _spread (Variables|Default|GetSpread))
  (for _index (range 1 100)
    (bind _returnvalue (Game|SpawnActorfromClass "/Game/Blueprints/DeathParticleMesh_BP.DeathParticleMesh_BP_C" (Math|Transform|MakeTransform (.location SpawnTransform) (.rotation SpawnTransform) (Math|Vector|MakeVector _scale _scale _scale)) "Undefined" 0 0))
    (Physics|SetPhysicsLinearVelocity (Variables|/Game/Blueprints/DeathParticleMesh_BP.DeathParticleMesh_BP_C|GetCube _returnvalue) (* (* (Class|KismetMathLibrary|RandomUnitVectorinCone "0, 0,1.000000" 45.0) (Math|Random|RandomFloatinRange (* -1 _spread) _spread)) (Math|Vector|MakeVector 1.0 1.0 (Variables|Default|GetHeight))) false "None")
    (Class|PrimitiveComponent|SetPhysicsAngularVelocity (Variables|/Game/Blueprints/DeathParticleMesh_BP.DeathParticleMesh_BP_C|GetCube _returnvalue) (* (Math|Random|RandomUnitVector) 500) false "None")))