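; Crusher hazard that moves vertically in world space and carries a damage component.
; On BeginPlay it records its location, and a timeline with configurable speed and start time lerps the root toward a point offset on Z by Distance.
; The construction script assigns the Damager volume as the trigger of DamagableBP and sets the Stem's initial Z scale.
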(event EventBeginPlay
  (Variables|Default|SetCurrentLocation (Transformation|GetWorldLocation (Variables|Default|GetDefaultSceneRoot)))
  (Variables|Default|SetTargetLocation (+ (Variables|Default|GetCurrentLocation) (Math|Vector|MakeVector 0.0 0.0 (Variables|Default|GetDistance))))
  (Components|Timeline|SetPlayRate (Variables|Default|GetTimeline_0) (Variables|Default|GetSpeed))
  (bind _smooth (Timeline|Timeline_0 SetNewTime)
    (:Update
      (Transformation|SetWorldLocation (Variables|Default|GetDefaultSceneRoot) (Math|Vector|Lerp(Vector) (Variables|Default|GetCurrentLocation) (Variables|Default|GetTargetLocation) _smooth) false false))))

(fn ConstructionScript
  (bind _stem (Variables|Default|GetStem))
  (bind _relativescale3d (Variables|/Script/Engine.SceneComponent|GetRelativeScale3D _stem))
  (Variables|/Game/Blueprints/Damagable_BP.Damagable_BP_C|SetTriggerVolume (Variables|Default|GetDamagable_BP) (Variables|Default|GetDamager))
  (Transformation|SetRelativeScale3D _stem (Math|Vector|MakeVector (.x _relativescale3d) (.y _relativescale3d) (Variables|Default|GetStartStemScale))))