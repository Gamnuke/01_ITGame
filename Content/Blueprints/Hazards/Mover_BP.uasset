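; Mover_BP is a hazard actor that moves from its starting position along its forward vector by a set Distance.
; On BeginPlay it caches both endpoints and plays the VInterp timeline at a play rate set by Speed.
; Each update lerps the root's world location without sweeping, using either the timeline's Smooth or Linear track as chosen by SmoothMove.
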(event EventBeginPlay
  (bind _defaultsceneroot (Variables|Default|GetDefaultSceneRoot))
  (bind _returnvalue (Transformation|GetWorldLocation _defaultsceneroot))
  (Variables|Default|SetCurrentLocation _returnvalue)
  (Variables|Default|SetTargetLocation (+ _returnvalue (* (Math|Vector|GetForwardVector _defaultsceneroot) (Variables|Default|GetDistance))))
  (Components|Timeline|SetPlayRate (Variables|Default|GetVInterp) (Variables|Default|GetSpeed))
  (bind (_direction _smooth _linear) (Timeline|VInterp PlayFromStart)
    (:Update
      (Transformation|SetWorldLocation (Variables|Default|GetDefaultSceneRoot) (Math|Vector|Lerp(Vector) (Variables|Default|GetCurrentLocation) (Variables|Default|GetTargetLocation) (select (Variables|Default|GetSmoothMove) _smooth _linear)) false false))))

(fn ConstructionScript)