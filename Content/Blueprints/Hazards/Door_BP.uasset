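; Hazard door Blueprint that opens or closes by scaling its DoorGraphics component on the Z axis.
; The OpenDoor event plays the DoorOpen timeline forward or in reverse according to the OpenDoor flag, then clears CanMove, which this graph never resets.
; BeginPlay applies Speed as the timeline play rate and, when the flag is false, sets the initial scale from the timeline's current value.
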(event Custom|OpenDoor
  (bind _doorgraphics (Variables|Default|GetDoorGraphics))
  (bind _relativescale3d (Variables|/Script/Engine.SceneComponent|GetRelativeScale3D _doorgraphics))
  (if (Variables|Default|GetCanMove)
    (Variables|Default|SetCanMove false)
    (if (Variables|Default|GetOpen%20Door?)
      (bind _dooropen (Timeline|DoorOpen PlayFromStart)
        (:Update
          (Transformation|SetRelativeScale3D _doorgraphics (Math|Vector|MakeVector (.x _relativescale3d) (.y _relativescale3d) _dooropen))))
      (else
        (Timeline|DoorOpen ReverseFromEnd)))))

(event EventBeginPlay
  (bind _doorgraphics (Variables|Default|GetDoorGraphics))
  (bind _relativescale3d (Variables|/Script/Engine.SceneComponent|GetRelativeScale3D _doorgraphics))
  (Components|Timeline|SetPlayRate (Variables|Default|GetDoorOpen) (Variables|Default|GetSpeed))
  (if (not (Variables|Default|GetOpen%20Door?))
    (Transformation|SetRelativeScale3D _doorgraphics (Math|Vector|MakeVector (.x _relativescale3d) (.y _relativescale3d) (stale Custom|OpenDoor _dooropen)))))

(fn ConstructionScript)