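; Player character for a side-scrolling game that moves along X, jumps, and on damage is destroyed and respawned through GameMode_BP.
; Tick interpolates movement offsets and facing, zeroes the physics box's horizontal velocity, and drives zoom plus a smoothed, absolute-transform spring-arm camera.
; Jumping sets vertical velocity when JumpVolume has overlaps, with timelines animating jump rotation and movement bobbing.
; A line-trace landing correction is present but unconnected.
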(event Custom|DamagePlayer
  ;[1 1 1] Inflicts damage and spawns new character when dead
  (Actor|DestroyActor)
  (bind _asgame_mode_bp (Utilities|Casting|CastToGameMode_BP (Game|GetGameMode)))
  (Default|SpawnCharacter _asgame_mode_bp))

(event EventBeginPlay
  (bind _springarm (Variables|Default|GetSpringArm))
  ;[1 1 1] Makes camera not relative to parent
  (Transformation|SetAbsolute _springarm true true false)
  (Transformation|SetWorldLocation _springarm (Transformation|GetWorldLocation (Variables|Default|GetBox)) false false))

(event EventTick
  (params (DeltaSeconds :type Float%20%28single-precision%29))
  (bind _returnvalue (Transformation|GetActorLocation))
  (bind _returnvalue_2 (Input|AxisValues|GetHorizontalMovement))
  (bind _springarm (Variables|Default|GetSpringArm))
  (bind _springarm_2 (Variables|Default|GetSpringArm))
  (bind _zoomlimit (Variables|Camera|GetZoomLimit))
  (bind (_x _y) (Math|Vector2D|BreakVector2D _zoomlimit))
  ;[1 1 1] Zoom
  (Variables|/Script/Engine.SpringArmComponent|SetTargetArmLength _springarm (Math|Float|Clamp(Float) (+ (* (Class|Actor|GetInputAxisKeyValue) (Variables|Camera|GetZoomMultiplier) -1.0) (Variables|/Script/Engine.SpringArmComponent|GetTargetArmLength _springarm)) _x _y))
  ;[1 1 1] Horizontal movement
  (bind _output_get (Variables|Movement|SetCurrentSmoothValue (Math|Interpolation|FInterpTo (Variables|Movement|GetCurrentSmoothValue) (* DeltaSeconds _returnvalue_2 (Variables|Movement|GetMoveMultiplier)) DeltaSeconds (Variables|Movement|GetMoveSmoothTime))))
  (Transformation|AddActorWorldOffset (Math|Vector|MakeVector _output_get 0.0 0.0) false true)
  ;[1 1 1] Smoothly Rotates character to direction of travel
  (if (!= _returnvalue_2 0.0)
    (Variables|Movement|SetInitialLookDirection _returnvalue_2)
    (Variables|Movement|SetCurrentHorizonMove _returnvalue_2))
  (Transformation|SetActorRotation (Math|Rotator|MakeRotator (Math|Conversions|ToFloat(Integer) (Math|Float|Round (Math|Float|Absolute(Float) (.roll (Math|Interpolation|RInterpTo (Transformation|GetActorRotation) (Math|Rotator|FindLookatRotation _returnvalue (+ (Math|Vector|MakeVector (Variables|Movement|GetCurrentHorizonMove) 0.0 0.0) _returnvalue)) DeltaSeconds (Variables|Movement|GetRotationSmoothTime)))))) (Math|Conversions|ToFloat(Integer) (Math|Float|Round (Math|Float|Absolute(Float) (.pitch (Math|Interpolation|RInterpTo (Transformation|GetActorRotation) (Math|Rotator|FindLookatRotation _returnvalue (+ (Math|Vector|MakeVector (Variables|Movement|GetCurrentHorizonMove) 0.0 0.0) _returnvalue)) DeltaSeconds (Variables|Movement|GetRotationSmoothTime)))))) (Math|Conversions|ToFloat(Integer) (Math|Float|Round (Math|Float|Absolute(Float) (.yaw (Math|Interpolation|RInterpTo (Transformation|GetActorRotation) (Math|Rotator|FindLookatRotation _returnvalue (+ (Math|Vector|MakeVector (Variables|Movement|GetCurrentHorizonMove) 0.0 0.0) _returnvalue)) DeltaSeconds (Variables|Movement|GetRotationSmoothTime))))))) true)
  ;[1 1 1] Camera movement smoothener
  (Transformation|SetWorldLocation _springarm_2 (Math|Interpolation|VInterpTo (Transformation|GetWorldLocation _springarm_2) (+ (Transformation|GetWorldLocation (Variables|Default|GetBox)) "0, 0,50.000000") DeltaSeconds 4.0) false false)
  ;[1 1 1] Horizontal force correction
  (bind _returnvalue_3 (Physics|GetPhysicsLinearVelocity (Variables|Default|GetBox) "None"))
  (Class|PrimitiveComponent|SetAllPhysicsLinearVelocity (Variables|Default|GetBox) (Math|Vector|MakeVector 0.0 0.0 (.z _returnvalue_3)) false)
  ;[1 1 1] Makes character bob when moving
  (if (!= 0.0 _returnvalue_2)
    (bind _bobbing (Timeline|Character%20bobbing Play)
      (:Update
        (Transformation|SetWorldScale3D (Variables|Default|GetGraphics) (Math|Vector|MakeVector 1.0 1.0 _bobbing))))
    (else
      (Timeline|Character%20bobbing Stop))))

(event Input|ActionEvents|InputActionJump
  (params (Key :type Key%20Structure))
  ;[1 1 1] Makes the player jump when touching the ground
  (:Pressed
    (if (> (Utilities|Array|Length (Collision|GetOverlappingActors (Variables|Default|GetJumpVolume) 0 :!class /Script/Engine.PrimitiveComponent)) 0)
      (Physics|SetPhysicsLinearVelocity (Variables|Default|GetBox) (Math|Vector|MakeVector 0.0 0.0 (Variables|Movement|GetJumpForce)) false "None")
      ;[1 1 1] Jump rotation
      (bind _rotation (Timeline|JumpRotation PlayFromStart)
        (:Update
          (Transformation|SetWorldRotation (Variables|Default|GetGraphicHolder) (Math|Rotator|MakeRotator 0.0 (* (Input|AxisValues|GetHorizontalMovement) _rotation -1.0) 0.0) false false))))))

(fn ConstructionScript)