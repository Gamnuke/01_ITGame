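; Liquid actor that moves vertically after the player and serves as a damage trigger through its DamagableBP.
; Each Tick, while a player pawn exists, it offsets its Z at a rate of one tenth of the gap to a point just above the pawn, so it moves faster when farther away and can also descend.
; The construction script sets its StaticMesh as DamagableBP's TriggerVolume; RisingSpeed is unused.
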(event EventTick
  (params (DeltaSeconds :type Float%20%28single-precision%29))
  (bind _returnvalue (Game|Player|GetPlayerPawn 0))
  (if (not (== _returnvalue 0))
    (Transformation|AddActorWorldOffset (Math|Vector|MakeVector 0.0 0.0 (* (/ (.z (- (+ (Transformation|GetActorLocation _returnvalue) "0, 0,100.000000") (Transformation|GetActorLocation))) 1e+01) DeltaSeconds)))))

(fn ConstructionScript
  (Variables|/Game/Blueprints/Damagable_BP.Damagable_BP_C|SetTriggerVolume (Variables|Default|GetDamagable_BP) (Variables|Default|GetStaticMesh)))