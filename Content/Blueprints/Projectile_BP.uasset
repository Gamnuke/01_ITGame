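; Projectile actor that flies straight without a movement component, driven by Tick.
; Each frame it line-traces the Visibility channel from the Bullet component along its forward vector, only one unit ahead regardless of Speed.
; With no hit, it offsets Bullet forward by Speed times delta time, without sweep.
; On a hit, it moves the actor to the impact point, prints a debug string and destroys itself.
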(event EventTick
  (params (DeltaSeconds :type Float%20%28single-precision%29))
  (bind _bullet (Variables|Default|GetBullet))
  (bind _bullet_2 (Variables|Default|GetBullet))
  (bind _returnvalue (Transformation|GetWorldLocation _bullet))
  (bind (_outhit _returnvalue_2) (Collision|LineTraceByChannel _returnvalue (+ _returnvalue (Math|Vector|GetForwardVector _bullet)) "TraceTypeQuery1" false 0 "None"))
  (if _returnvalue_2
    (Transformation|SetActorLocation (|GetImpactPoint _outhit) false false)
    (Development|PrintString "Hello")
    (Actor|DestroyActor)
    (else
      (Transformation|AddWorldOffset _bullet_2 (* (Math|Vector|GetForwardVector _bullet_2) (* (Variables|Default|GetSpeed) DeltaSeconds)) false false))))

(fn ConstructionScript)