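; Checkpoint actor that moves the level's respawn point when the player character reaches it.
; On BeginPlay it binds to its Box's begin-overlap event and responds only to Character_BP.
; An overlap turns its light and mesh components plasma green, then moves the PlayerStart referenced by GameMode_BP to the box's world X and Z, without passing Y.
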(event Custom|OnComponentBeginOverlap_Event_0
  (params (OverlappedComponent :type Primitive%20Component%20Object%20Reference) (OtherActor :type Actor%20Object%20Reference) (OtherComp :type Primitive%20Component%20Object%20Reference) (OtherBodyIndex :type Integer) (bFromSweep :type Boolean) (SweepResult :type Hit%20Result%20Structure%20%28by%20ref%29))
  (bind _box (Variables|Default|GetBox))
  (bind _returnvalue (Transformation|GetWorldLocation _box))
  (Utilities|Casting|CastToCharacter_BP OtherActor)
  (for _array_element (Utilities|Array|MakeArray (Variables|Default|GetLight2) (Variables|Default|GetStaticMesh2) (Variables|Default|GetStaticMesh3) (Variables|Default|GetStaticMesh4) (Variables|Default|GetStaticMesh5) (Variables|Default|GetLight))
    (Rendering|Material|SetMaterial _array_element 0 "/Game/Materials/PlasmaGreen_M.PlasmaGreen_M"))
  (bind _asgame_mode_bp (Utilities|Casting|CastToGameMode_BP (Game|GetGameMode)))
  (Transformation|SetActorLocation (Variables|/Game/Blueprints/GameMode_BP.GameMode_BP_C|GetPlayerStart _asgame_mode_bp) (Math|Vector|MakeVector (.x _returnvalue) 0.0 (.z _returnvalue)) false false))

(event EventBeginPlay
  (Collision|AssignOnComponentBeginOverlap (Variables|Default|GetBox) (delegate Custom|OnComponentBeginOverlap_Event_0)))

(fn ConstructionScript)